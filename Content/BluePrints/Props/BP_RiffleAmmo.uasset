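; BP_RiffleAmmo is an ammo pickup prop that adds reserve rounds for a specific weapon class.
; A sphere overlap shows an interact widget while the FPS player character is in range and removes it on exit.
; On Interact, if the player's Weapon child actor class matches REFBaseWeapon, it adds Ammo to that weapon's MaxAmmo, clears the widget and destroys itself.
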(event `self.ReceiveBeginPlay`
  (bind _asbp_fpsplayer_character (cast `/Game/BluePrints/BP_FPSPlayerCharacter` (`GameplayStatics.GetPlayerCharacter` 0)))
  (set `self.Player Reference` _asbp_fpsplayer_character))

(event `self.Interact`
  (bind _ref_interactwidget (`self.REF InteractWidget`))
  (bind _player_reference (`self.Player Reference`))
  (bind _weaponreference (`/Game/BluePrints/BP_FPSPlayerCharacter.WeaponReference` _player_reference))
  (if (== (`ChildActorComponent.ChildActorClass` (`/Game/BluePrints/BP_FPSPlayerCharacter.Weapon` _player_reference)) (`self.REF BaseWeapon`))
    (set `/Game/BluePrints/Weapons/BP_BaseWeapon.MaxAmmo` (+ (`/Game/BluePrints/Weapons/BP_BaseWeapon.MaxAmmo` _weaponreference) (`self.Ammo`)) _weaponreference)
    (`/Engine/EditorBlueprintResources/StandardMacros.IsValid` _ref_interactwidget
      (:`Is Valid`
        (`Widget.RemoveFromParent` _ref_interactwidget))
      (:`Is Not Valid`
        _))
    (`self.K2_DestroyActor`)))

(event `self.Sphere.OnComponentBeginOverlap`
  (params (OverlappedComponent :type "PrimitiveComponent Object Reference") (OtherActor :type "Actor Object Reference") (OtherComp :type "PrimitiveComponent Object Reference") (OtherBodyIndex :type Integer) (bFromSweep :type Boolean) (SweepResult :type "HitResult Structure (by ref)"))
  (cast `/Game/BluePrints/BP_FPSPlayerCharacter` OtherActor)
  (bind _returnvalue (`|CreateWidget` "/Game/UI/BPW_InteractWidget.BPW_InteractWidget_C"))
  (bind _output_get (set `self.REF InteractWidget` _returnvalue))
  (`UserWidget.AddToViewport` _output_get 0))

(event `self.Sphere.OnComponentEndOverlap`
  (params (OverlappedComponent :type "PrimitiveComponent Object Reference") (OtherActor :type "Actor Object Reference") (OtherComp :type "PrimitiveComponent Object Reference") (OtherBodyIndex :type Integer))
  (bind _ref_interactwidget (`self.REF InteractWidget`))
  (cast `/Game/BluePrints/BP_FPSPlayerCharacter` OtherActor)
  (`/Engine/EditorBlueprintResources/StandardMacros.IsValid` _ref_interactwidget
    (:`Is Valid`
      (`Widget.RemoveFromParent` _ref_interactwidget))))

(fn `UserConstructionScript`)