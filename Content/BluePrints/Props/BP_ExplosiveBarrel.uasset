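; Explosive barrel prop that detonates when its health runs out from incoming damage.
; AnyDamage reduces Health, and at zero it spawns an explosion emitter and sphere-traces for pawns within the explosive radius.
; Each hit pawn receives barrel explosion damage before the barrel destroys itself, with the trace drawing debug for a duration.
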(event `self.ReceiveAnyDamage`
  (params (Damage :type "Float (single-precision)") (DamageType :type "DamageType Object Reference") (InstigatedBy :type "Controller Object Reference") (DamageCauser :type "Actor Object Reference"))
  (bind _returnvalue (`self.K2_GetActorLocation`))
  (bind _output_get (set `self.Health` (- (`self.Health`) Damage)))
  (if (<= _output_get 0.0)
    (`GameplayStatics.SpawnEmitterAtLocation` "/Game/MilitaryWeapSilver/FX/P_Grenade_Explosion_01.P_Grenade_Explosion_01" (`self.K2_GetActorLocation`) (struct) (2.0 2.0 2.0))
    (bind _outhits (`KismetSystemLibrary.SphereTraceMultiForObjects` :`Start` _returnvalue :`End` _returnvalue :`Radius` (`self.ExplosiveRadius`) :`ObjectTypes` (`|MakeArray` "ObjectTypeQuery3" :!type "EObjectTypeQuery Enum") :`DrawDebugType` "ForDuration"))
    (for _array_element _outhits
      (`GameplayStatics.ApplyDamage` (`.HitActor` (`GameplayStatics.BreakHitResult` _array_element)) (`self.BarrelExplosiveDamage`)))
    (`self.K2_DestroyActor`)))

(fn `UserConstructionScript`)