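; BP_WeaponPickUp is a world weapon pickup that swaps its weapon with the one the FPS player is holding.
; On Interact it replaces the held main or secondary slot, spawning a new pickup in its place with the dropped weapon and ammo.
; It then refreshes the player's child-actor weapon, HUD and ammo, and destroys itself.
; The construction script picks the skeletal mesh from the stored weapon class's default name.
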(event `self.ReceiveBeginPlay`
  (bind _asbp_fpsplayer_character (cast `/Game/BluePrints/BP_FPSPlayerCharacter` (`GameplayStatics.GetPlayerCharacter` 0)))
  (set `self.REF FPS Player` _asbp_fpsplayer_character))

(event `/Game/BluePrints/Interface/BPI_Interaction.Interact`
  (bind _ref_fps_player (`self.REF FPS Player`))
  (bind (_weapon_struct_weapon _weapon_struct_currentammo _weapon_struct_maxammo) (break `/Game/BluePrints/Structure/BPS_WeaponStruct` (`self.Weapon Struct`)))
  (bind (_weapon_struct_weapon_2 _weapon_struct_currentammo_2 _weapon_struct_maxammo_2) (break `/Game/BluePrints/Structure/BPS_WeaponStruct` (`self.Weapon Struct`)))
  (bind _ref_fps_player_2 (`self.REF FPS Player`))
  (bind _weapon_struct_weapon_3 (break `/Game/BluePrints/Structure/BPS_WeaponStruct` (`self.Weapon Struct`)))
  (bind (_weapon_struct_weapon_4 _weapon_struct_currentammo_3 _weapon_struct_maxammo_3) (break `/Game/BluePrints/Structure/BPS_WeaponStruct` (`self.Weapon Struct`)))
  (bind _ref_fps_player_3 (`self.REF FPS Player`))
  (bind _ref_fps_player_4 (`self.REF FPS Player`))
  (bind (_weapon_struct_weapon_5 _weapon_struct_currentammo_4 _weapon_struct_maxammo_4) (break `/Game/BluePrints/Structure/BPS_WeaponStruct` (`self.Weapon Struct`)))
  (bind _ref_fps_player_5 (`self.REF FPS Player`))
  (bind _weapon_struct_weapon_6 (break `/Game/BluePrints/Structure/BPS_WeaponStruct` (`self.Weapon Struct`)))
  (bind _weaponreference (`/Game/BluePrints/BP_FPSPlayerCharacter.WeaponReference` _ref_fps_player_5))
  (bind _weaponreference_2 (`/Game/BluePrints/BP_FPSPlayerCharacter.WeaponReference` _ref_fps_player_2))
  (bind _mainweapon_weapon (break `/Game/BluePrints/Structure/BPS_WeaponStruct` (`/Game/BluePrints/BP_FPSPlayerCharacter.MainWeapon` _ref_fps_player_4)))
  (bind _secondaryweapon_weapon (break `/Game/BluePrints/Structure/BPS_WeaponStruct` (`/Game/BluePrints/BP_FPSPlayerCharacter.SecondaryWeapon` _ref_fps_player_3)))
  (bind _weaponreference_3 (`/Game/BluePrints/BP_FPSPlayerCharacter.WeaponReference` _ref_fps_player_4))
  (bind _mainweapon_weapon_2 (break `/Game/BluePrints/Structure/BPS_WeaponStruct` (`/Game/BluePrints/BP_FPSPlayerCharacter.MainWeapon` _ref_fps_player)))
  (bind _weaponreference_4 (`/Game/BluePrints/BP_FPSPlayerCharacter.WeaponReference` _ref_fps_player_3))
  (if (== (`ChildActorComponent.ChildActorClass` (`/Game/BluePrints/BP_FPSPlayerCharacter.Weapon` _ref_fps_player)) _mainweapon_weapon_2)
    ;[0 0 0] Weapon swap
    ;;[1 1 1] Swap main weapon
    (`|SpawnActorFromClass` "BP_WeaponPickUp_C" (`self.GetTransform`) "Undefined" "MultiplyWithRoot" null (make `/Game/BluePrints/Structure/BPS_WeaponStruct` _mainweapon_weapon (`/Game/BluePrints/Weapons/BP_BaseWeapon.CurrentAmmo` _weaponreference_3) (`/Game/BluePrints/Weapons/BP_BaseWeapon.MaxAmmo` _weaponreference_3)) null)
    (set `/Game/BluePrints/BP_FPSPlayerCharacter.MainWeapon` (make `/Game/BluePrints/Structure/BPS_WeaponStruct` _weapon_struct_weapon_2 _weapon_struct_currentammo_2 _weapon_struct_maxammo_2) (`self.REF FPS Player`))
    (`Widget.RemoveFromParent` (`/Game/BluePrints/BP_FPSPlayerCharacter.PlayerHUD_REF` _ref_fps_player_2))
    (`ChildActorComponent.SetChildActorClass` (`/Game/BluePrints/BP_FPSPlayerCharacter.Weapon` _ref_fps_player_2) _weapon_struct_weapon_3)
    (`/Game/BluePrints/BP_FPSPlayerCharacter.Select Weapon` _ref_fps_player_2)
    (`/Game/BluePrints/BP_FPSPlayerCharacter.Set Player HUD` _ref_fps_player_2)
    (`/Game/BluePrints/BP_FPSPlayerCharacter.maintain ammo Inf` _ref_fps_player_2)
    (set `/Game/BluePrints/Weapons/BP_BaseWeapon.CurrentAmmo` _weapon_struct_currentammo_3 _weaponreference_2)
    (set `/Game/BluePrints/Weapons/BP_BaseWeapon.MaxAmmo` _weapon_struct_maxammo_3 _weaponreference_2)
    (`self.K2_DestroyActor`)
    (else
      ;;[1 1 1] Swap Second weapon
      (`|SpawnActorFromClass` "BP_WeaponPickUp_C" (`self.GetTransform`) "Undefined" "MultiplyWithRoot" null (make `/Game/BluePrints/Structure/BPS_WeaponStruct` _secondaryweapon_weapon (`/Game/BluePrints/Weapons/BP_BaseWeapon.CurrentAmmo` _weaponreference_4) (`/Game/BluePrints/Weapons/BP_BaseWeapon.MaxAmmo` _weaponreference_4)) null)
      (set `/Game/BluePrints/BP_FPSPlayerCharacter.SecondaryWeapon` (make `/Game/BluePrints/Structure/BPS_WeaponStruct` _weapon_struct_weapon_5 _weapon_struct_currentammo_4 _weapon_struct_maxammo_4) (`self.REF FPS Player`))
      (`Widget.RemoveFromParent` (`/Game/BluePrints/BP_FPSPlayerCharacter.PlayerHUD_REF` _ref_fps_player_5))
      (`ChildActorComponent.SetChildActorClass` (`/Game/BluePrints/BP_FPSPlayerCharacter.Weapon` _ref_fps_player_5) _weapon_struct_weapon_6)
      (`/Game/BluePrints/BP_FPSPlayerCharacter.Select Weapon` _ref_fps_player_5)
      (`/Game/BluePrints/BP_FPSPlayerCharacter.Set Player HUD` _ref_fps_player_5)
      (`/Game/BluePrints/BP_FPSPlayerCharacter.maintain ammo Inf` _ref_fps_player_5)
      (set `/Game/BluePrints/Weapons/BP_BaseWeapon.CurrentAmmo` _weapon_struct_currentammo _weaponreference)
      (set `/Game/BluePrints/Weapons/BP_BaseWeapon.MaxAmmo` _weapon_struct_maxammo _weaponreference)
      (`self.K2_DestroyActor`))))

(fn `UserConstructionScript`
  (bind _weapon_struct_weapon (break `/Game/BluePrints/Structure/BPS_WeaponStruct` (`self.Weapon Struct`)))
  (switch `string` (`KismetTextLibrary.Conv_TextToString` (`.WeaponName` (defaults `Object` _weapon_struct_weapon)))
    (:`M1911`
      (`SkeletalMeshComponent.SetSkeletalMeshAsset` (`self.SkeletalMesh`) "/Game/MilitaryWeapSilver/Weapons/Pistols_A.Pistols_A"))
    (:`FN15A3`
      (`SkeletalMeshComponent.SetSkeletalMeshAsset` (`self.SkeletalMesh`) "/Game/MilitaryWeapSilver/Weapons/Assault_Rifle_A.Assault_Rifle_A"))
    (:`M37`
      (`SkeletalMeshComponent.SetSkeletalMeshAsset` (`self.SkeletalMesh`) "/Game/MilitaryWeapSilver/Weapons/Shotgun_A.Shotgun_A"))))