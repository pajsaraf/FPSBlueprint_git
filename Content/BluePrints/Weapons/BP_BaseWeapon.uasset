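; Base weapon Blueprint providing hitscan firing, iron sights and reloading, with empty shooting start/stop events.
; Iron sights blend the view to the weapon's own camera, while Tick syncs the player's camera to control rotation.
; FireWeapon line-traces from the active camera, spends ammo, shakes the camera, emits noise, then damages Enemy-tagged actors with blood effects or leaves bullet-hole decals.
; ReloadSystem refills the magazine from reserve ammo.
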(event `self.ReceiveTick`
  (params (DeltaSeconds :type "Float (single-precision)"))
  (if (`self.bIsIronSights?`)
    (`SceneComponent.K2_SetWorldRotation` (`/Game/BluePrints/BP_FPSPlayerCharacter.Camera` (`self.PlayerReference`)) (`Controller.GetControlRotation` (`GameplayStatics.GetPlayerController` 0)) false false)))

(event `Start Shooting`)

(event `StopShooting`)

(event `Start Ironsights`
  ;[1 1 1] Switch to gun camera  iron sights
  (set `self.bIsIronSights?` true)
  (`PlayerController.SetViewTargetWithBlend` (`GameplayStatics.GetPlayerController` 0) self 0.16 "VTBlend_Linear" 0.0 false))

(event `Stop Ironsights`
  ;[1 1 1] Switch to player camera
  (set `self.bIsIronSights?` false)
  (`PlayerController.SetViewTargetWithBlend` (`GameplayStatics.GetPlayerController` 0) (`GameplayStatics.GetPlayerCharacter` 0) 0.16 "VTBlend_Linear" 0.0 false))

(fn `FireWeapon`
  (bind _playerreference (`self.PlayerReference`))
  (bind _returnvalue (select `bool` (`self.bIsIronSights?`) :`false` (`/Game/BluePrints/BP_FPSPlayerCharacter.Camera` (`self.PlayerReference`)) :`true` (`self.Camera`)))
  (bind _returnvalue_2 (`SceneComponent.K2_GetComponentLocation` _returnvalue))
  (if (> (`self.CurrentAmmo`) 0)
    (set `self.bCanPlayAnimation?` true)
    (`/Game/BluePrints/BP_FPSPlayerCharacter.CameraShake Fire` (`self.PlayerReference`))
    (bind _outhit (`KismetSystemLibrary.LineTraceSingle` _returnvalue_2 (+ _returnvalue_2 (* (`SceneComponent.GetForwardVector` _returnvalue) 3000.0)) "TraceTypeQuery1"))
    (`/Engine/EditorBlueprintResources/StandardMacros.DecrementInt` (`self.CurrentAmmo`)
      (:`  `
        (`PawnNoiseEmitterComponent.MakeNoise` (`/Game/BluePrints/BP_FPSPlayerCharacter.PawnNoiseEmitter` _playerreference) _playerreference 1.0 (`self.K2_GetActorLocation` _playerreference))
        (bind (_bblockinghit _binitialoverlap _time _distance _location _impactpoint _normal _impactnormal _physmat _hitactor) (`GameplayStatics.BreakHitResult` _outhit))
        (`/Engine/EditorBlueprintResources/StandardMacros.IsValid` _hitactor
          (:`Is Valid`
            (if (`self.ActorHasTag` _hitactor "Enemy")
              (`GameplayStatics.ApplyDamage` _hitactor (`self.Base Damage`))
              (`GameplayStatics.SpawnEmitterAtLocation` "/Game/Realistic_Starter_VFX_Pack_Vol2/Particles/Blood/P_Blood_Splat_Cone.P_Blood_Splat_Cone" _location)
              (else
                (`GameplayStatics.SpawnDecalAtLocation` "/Game/Images/M_BulletHole.M_BulletHole" (6.0 6.0 6.0) _location (`KismetMathLibrary.Conv_VectorToRotator` _impactnormal) 30.0)
                (`GameplayStatics.SpawnEmitterAtLocation` "/Game/Realistic_Starter_VFX_Pack_Vol2/Particles/Hit/P_Default.P_Default" _location)))))))
    (else
      (set `self.bCanPlayAnimation?` false))))

(fn `ReloadSystem`
  (locals (L_AmmoDifference :type Integer))
  (bind _output_get (set `local.L_AmmoDifference` (- (`self.MagazineSize`) (`self.CurrentAmmo`))))
  (if (>= (`self.MaxAmmo`) _output_get)
    (set `self.CurrentAmmo` (`self.MagazineSize`))
    (set `self.MaxAmmo` (- (`self.MaxAmmo`) (`local.L_AmmoDifference`)))
    (else
      (set `self.CurrentAmmo` (+ (`self.CurrentAmmo`) (`self.MaxAmmo`)))
      (set `self.MaxAmmo` 0))))

(fn `UserConstructionScript`)