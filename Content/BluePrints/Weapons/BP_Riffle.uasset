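; BP_Riffle is an automatic rifle weapon that fires only while aiming down iron sights.
; StartShooting fires once and, if animation is allowed, plays the gun animation and starts a looping FireRate timer.
; Each timer tick runs FireRifle, which calls FireWeapon and plays gun and first-person hands animations.
; Shooting stops by clearing the timer, including when a tick finds aiming ended or animation disallowed.
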(event `self.Start Shooting`
  (if (`self.bIsIronSights?`)
    (`self.FireWeapon`)
    (if (`self.bCanPlayAnimation?`)
      (`SkeletalMeshComponent.PlayAnimation` (`self.GunMesh`) "/Game/MilitaryWeapSilver/Weapons/Animations/Fire_Rifle_W.Fire_Rifle_W" false)
      (bind _returnvalue (`KismetSystemLibrary.K2_SetTimerDelegate` (delegate `Fire Rifle`) (`self.FireRate`) true))
      (set `self.FireEvent` _returnvalue))
    (else
      (`self.StopShooting`))))

(event `Fire Rifle`
  (if (`self.bIsIronSights?`)
    (`self.FireWeapon`)
    (if (`self.bCanPlayAnimation?`)
      (`SkeletalMeshComponent.PlayAnimation` (`self.GunMesh`) "/Game/MilitaryWeapSilver/Weapons/Animations/Fire_Rifle_W.Fire_Rifle_W" false)
      (`|PlayMontage` (`/Game/BluePrints/BP_FPSPlayerCharacter.FPSHands_SkeletalMesh` (`self.PlayerReference`)) "/Game/Man/Demo/Animations/FiringRifle_UE_Montage.FiringRifle_UE_Montage")
      (else
        (`self.StopShooting`)))
    (else
      (`self.StopShooting`))))

(event `self.StopShooting`
  (`KismetSystemLibrary.K2_ClearAndInvalidateTimerHandle` (`self.FireEvent`)))

(fn `UserConstructionScript`
  (`parent.UserConstructionScript`))