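; Zombie enemy Blueprint that roams randomly, chases pawns it sees and dies when its health runs out.
; Roam loops AI moves to random reachable points with a short pause after each successful arrival.
; PawnSensing sightings start a chase, and a retriggerable delay returns it to roaming once sightings stop.
; Lethal damage sets a dead flag, stops movement, disables capsule collision and plays a random falling montage.
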(event `self.ReceiveBeginPlay`
  (`self.ZombieSpeed`)
  (`self.Roam`))

(event `Roam`
  ;[1 1 1] Roam randomly
  (if (not (or (`self.bSeePlayer?`) (`self.bIsDead?`))) :!label _label
    (`|AIMoveTo` self (`NavigationSystemV1.K2_GetRandomReachablePointInRadius` (`self.K2_GetActorLocation`) 500.0 null null) null
      (:`OnSuccess`
        (`KismetSystemLibrary.Delay` 3.0)
        (goto _label)))))

(event `self.PawnSensing.OnSeePawn`
  (params (Pawn :type "Pawn Object Reference"))
  ;[1 1 1] Visual detection
  (if (not (`self.bIsDead?`))
    (set `self.bSeePlayer?` true)
    (`|ExecutionSequence`
      (:`then_0`
        (`|AIMoveTo` self (0.0 0.0 0.0) Pawn))
      (:`then_1`
        (`KismetSystemLibrary.RetriggerableDelay` 3.0)
        (set `self.bSeePlayer?` false)
        (`self.Roam`)))))

(event `ZombieSpeed`
  ;[1 1 1] Speed
  (set `CharacterMovementComponent.MaxWalkSpeed` (`self.Zombie Speed`) (`self.CharacterMovement`)))

(event `self.ReceiveAnyDamage`
  (params (Damage :type "Float (single-precision)") (DamageType :type "DamageType Object Reference") (InstigatedBy :type "Controller Object Reference") (DamageCauser :type "Actor Object Reference"))
  (bind _output_get (set `self.Health` (- (`self.Health`) Damage)))
  (if (<= _output_get 0.0)
    (`/Engine/EditorBlueprintResources/StandardMacros.DoOnce` false
      (:`Completed`
        (set `self.bIsDead?` true)
        (`MovementComponent.StopMovementImmediately` (`self.CharacterMovement`))
        (`PrimitiveComponent.SetCollisionEnabled` (`self.CapsuleComponent`) "NoCollision")
        (switch `int` (`KismetMathLibrary.RandomIntegerInRange` 0 1)
          (:`0`
            (`self.PlayAnimMontage` "/Game/BluePrints/Enemies/Zombie/animations/Zombie_Z_FallingBack_Montage.Zombie_Z_FallingBack_Montage"))
          (:`1`
            (`self.PlayAnimMontage` "/Game/BluePrints/Enemies/Zombie/animations/Zombie_Z_FallingForward_Montage.Zombie_Z_FallingForward_Montage")))))))

(fn `UserConstructionScript`)